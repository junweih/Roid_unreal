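; Global Blueprint actor that periodically spawns asteroids and keeps the player's score.
; A looping timer started on BeginPlay spawns a small batch of Asteroid actors at random X/Y positions on the Z=0 plane.
; Spawn bounds come from deprojecting the viewport-size screen corner to world space, scaled and mirrored around the origin.
; Each asteroid's AsteroidHit event is bound to IncrementScore, which adds points to Score.
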(event Custom|EventSpawn
  (bind _returnvalue (Game|GetPlayerController 0))
  (bind _returnvalue_2 (Viewport|GetViewportSize))
  (bind _worldposition (Class|GameplayStatics|DeprojectScreentoWorld _returnvalue _returnvalue_2))
  (bind _returnvalue_3 (* _worldposition 2e+01))
  (bind (_x _y) (Math|Vector|BreakVector _returnvalue_3))
  (for _index (range 0 2)
    (bind _returnvalue_4 (Game|SpawnActorfromClass "/Game/BluePrints/Asteroid.Asteroid_C" (Math|Transform|MakeTransform (Math|Vector|MakeVector (Math|Random|RandomFloatinRange (* _x -1.0) _x) (Math|Random|RandomFloatinRange (* _y -1.0) _y) 0.0)) "Undefined" 0 0))
    (EventDispatchers|BindEventtoAsteroidHit _returnvalue_4 (delegate Custom|IncrementScore))))

(event Custom|IncrementScore
  (Variables|Default|SetScore (+ (Variables|Default|GetScore) 2)))

(event EventBeginPlay
  (Utilities|Time|SetTimerbyEvent (delegate Custom|EventSpawn) 5.0 true))

(fn ConstructionScript)